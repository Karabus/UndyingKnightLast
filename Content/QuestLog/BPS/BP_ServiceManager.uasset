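; BP_ServiceManager is a quest-system facade that exposes a single set of entry points to the quest log.
; Its events forward starting, auto-starting and objective completion, plus active widget updates, to a QuestManager reference.
; Getter functions return the active quests, completed quests and active widget from that manager, and the Blueprint adds no logic of its own.
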(event `/Game/QuestLog/Interfaces/INT_ServiceManager.SM_StartQuest`
  (params (Quest :type Name))
  (`/Game/QuestLog/Interfaces/INT_QuestManager.QM_StartQuest` (`self.QuestManager`) Quest))

(event `/Game/QuestLog/Interfaces/INT_ServiceManager.SM_CompleteObjective`
  (params (QuestID :type Name) (ObjectiveID :type Name))
  (`/Game/QuestLog/Interfaces/INT_QuestManager.QM_CompleteObjective` (`self.QuestManager`) QuestID ObjectiveID))

(event `/Game/QuestLog/Interfaces/INT_ServiceManager.SM_AutoStartQuests`
  (`/Game/QuestLog/Interfaces/INT_QuestManager.QM_AutoStartQuest` (`self.QuestManager`)))

(event `/Game/QuestLog/Interfaces/INT_ServiceManager.SM_SetActiveWidget`
  (params (Widget :type "Widget Object Reference"))
  (message `/Game/QuestLog/Interfaces/INT_QuestManager.QM_UpdateActiveWidget` (`self.QuestManager`) Widget))

(fn `SM_GetActiveQuests`
  (returns (ActiveQuests :type "Array of /Game/QuestLog/Structs/S_QuestData Structure"))
  (bind _activequests (`/Game/QuestLog/Interfaces/INT_QuestManager.QM_GetActiveQuests` (`self.QuestManager`)))
  (return _activequests))

(fn `SM_GetActiveWidget`
  (returns (Widget :type "Widget Object Reference"))
  (bind _widget (`/Game/QuestLog/Interfaces/INT_QuestManager.QM_GetActiveWidget` (`self.QuestManager`)))
  (return _widget))

(fn `SM_GetCompletedQuests`
  (returns (CompletedQuests :type "Array of /Game/QuestLog/Structs/S_QuestData Structure"))
  (bind _completedquests (`/Game/QuestLog/Interfaces/INT_QuestManager.QM_GetCompletedQuests` (`self.QuestManager`)))
  (return _completedquests))

(fn `UserConstructionScript`)