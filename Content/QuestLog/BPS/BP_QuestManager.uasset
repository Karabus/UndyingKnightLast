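; Quest manager that starts quests, tracks objective completion and stores active and completed quests.
; Quests load from DT_quest by ID, including those flagged AutoStart, into ActiveQuests and a QuestProgress count map.
; Completing an objective rewrites the nested quest structs, bumps progress and, if all objectives are done, moves the quest to CompletedQuests.
; QM-prefixed events and getters expose this, with popup widgets announcing each start and completion.
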(event `/Game/QuestLog/Interfaces/INT_QuestManager.QM_StartQuest`
  (params (QuestID :type Name))
  (`self.StartQuest` QuestID))

(event `/Game/QuestLog/Interfaces/INT_QuestManager.QM_CompleteObjective`
  (params (QuestID :type Name) (ObjectID :type Name))
  (bind _output (`self.CompleteObjective` QuestID ObjectID))
  (if _output
    (`self.CompleteQuest` QuestID)))

(event `/Game/QuestLog/Interfaces/INT_QuestManager.QM_AutoStartQuest`
  (bind _outrownames (`DataTableFunctionLibrary.GetDataTableRowNames` "/Game/QuestLog/DataTable/DT_quest.DT_quest"))
  (for _array_element _outrownames
    (bind _returnvalue (`|GetDataTableRow` "/Game/QuestLog/DataTable/DT_quest.DT_quest" _array_element)
      (:`then`
        (bind (_questid _title _iscompleted _description _objectives _isrepeatable _autostart) (break `/Game/QuestLog/Structs/S_QuestData` _returnvalue))
        (if _autostart
          (`self.StartQuest` _questid))))))

(event `/Game/QuestLog/Interfaces/INT_QuestManager.QM_UpdateActiveWidget`
  (params (Widget :type "Widget Object Reference"))
  (set `self.ActiveWidget` Widget))

(fn `CheckIfQuestHasAllreadyStarted`
  (params (QuestId :type Name))
  (returns (CanStart :type Boolean))
  (for _array_element (`self.CompletedQuests`)
    (bind (_questid _title _iscompleted) (break `/Game/QuestLog/Structs/S_QuestData` _array_element))
    (if (and (not _iscompleted) (== _questid QuestId))
      (return false)))
  (for _array_element_2 (`self.ActiveQuests`)
    (if (== (`.QuestID_8_D0F829F54632ABB1EF689CB21D7A8BD5` (break `/Game/QuestLog/Structs/S_QuestData` _array_element_2)) QuestId)
      (return false)))
  (return true))

(fn `CheckQuestCompleted`
  (params (QuestID :type Name))
  (returns (Completed :type Boolean))
  (for _array_element (`self.ActiveQuests`)
    (if (== (`.QuestID_8_D0F829F54632ABB1EF689CB21D7A8BD5` (break `/Game/QuestLog/Structs/S_QuestData` _array_element)) QuestID)
      (for _array_element_2 (`.Objectives_27_DB1C4EAF429E6CEAACA8E8B6823740B7` (break `/Game/QuestLog/Structs/S_QuestData` _array_element))
        (if (not (`.IsCompleted_11_C69A1DC94C8425DD2F3154B9E59AFEC2` (break `/Game/QuestLog/Structs/S_QuestObjectives` _array_element_2)))
          (return false)))
      (return true)
      (else
        (return false)))))

(fn `CompleteObjective`
  (params (QuestID :type Name) (ObjectiveID :type Name))
  (returns (Output :type Boolean))
  (locals (TempProgress :type "Map of Name to Object Object Reference"))
  (bind (_value _returnvalue) (`BlueprintMapLibrary.Map_Find` (`local.TempProgress`) QuestID))
  (bind _completed (`self.UpdateObjectiveCompletion` QuestID ObjectiveID))
  (set `local.TempProgress` (`self.QuestProgress`))
  (if _returnvalue
    (bind _result (`/Engine/EditorBlueprintResources/StandardMacros.IncrementInt` _value)
      (:`  `
        (`BlueprintMapLibrary.Map_Add` (`local.TempProgress`) QuestID _result)
        (set `self.QuestProgress` (`local.TempProgress`))
        (bind _returnvalue_2 (`|GetDataTableRow` "/Game/QuestLog/DataTable/DT_quest.DT_quest" QuestID)
          (:`then`
            (for _array_element (`.Objectives_27_DB1C4EAF429E6CEAACA8E8B6823740B7` (break `/Game/QuestLog/Structs/S_QuestData` _returnvalue_2))
              (if (== (`.ObjectiveID_7_4D4F38A74C8366879E3010A40201A81D` (break `/Game/QuestLog/Structs/S_QuestObjectives` _array_element)) (`local.ObjectiveID`))
                (bind _returnvalue_3 (`|CreateWidget` "/Game/QuestLog/Widgets/WG_CompletedObjective.WG_CompletedObjective_C" null _array_element))
                (`UserWidget.AddToViewport` _returnvalue_3 0)))
            (return _completed)))))
    (else
      (return false))))

(fn `CompleteQuest`
  (params (QuestID :type Name))
  (for _array_element (`self.ActiveQuests`)
    (bind _questid (break `/Game/QuestLog/Structs/S_QuestData` _array_element))
    (if (== _questid QuestID)
      (bind _returnvalue (`|CreateWidget` "/Game/QuestLog/Widgets/WG_CompletedQuest.WG_CompletedQuest_C" null _array_element))
      (`UserWidget.AddToViewport` _returnvalue 0)
      (`KismetArrayLibrary.Array_Add` (`self.CompletedQuests`) _array_element)
      (`KismetArrayLibrary.Array_RemoveItem` (`self.ActiveQuests`) _array_element)
      (`BlueprintMapLibrary.Map_Remove` (`self.QuestProgress`) _questid)
      (return))))

(fn `QM_GetActiveQuests`
  (returns (ActiveQuests :type "Array of /Game/QuestLog/Structs/S_QuestData Structure"))
  (return (`self.ActiveQuests`)))

(fn `QM_GetActiveWidget`
  (returns (Widget :type "Widget Object Reference"))
  (return (`self.ActiveWidget`)))

(fn `QM_GetCompletedQuests`
  (returns (CompletedQuests :type "Array of /Game/QuestLog/Structs/S_QuestData Structure"))
  (return (`self.CompletedQuests`)))

(fn `StartQuest`
  (params (QuestID :type Name))
  (locals (TempProgress :type "Map of Name to Object Object Reference"))
  (bind _activequests (`self.ActiveQuests`))
  (bind _tempprogress (`local.TempProgress`))
  (`KismetSystemLibrary.PrintString` (`KismetStringLibrary.Concat_StrStr` "Start Quest:" (`KismetStringLibrary.Conv_NameToString` QuestID)))
  (bind _canstart (`self.CheckIfQuestHasAllreadyStarted` QuestID))
  (if _canstart
    (`KismetSystemLibrary.PrintString` "Este nezacal")
    (bind _returnvalue (`|GetDataTableRow` "/Game/QuestLog/DataTable/DT_quest.DT_quest" QuestID)
      (:`then`
        (`KismetArrayLibrary.Array_Add` _activequests _returnvalue)
        (`KismetSystemLibrary.PrintString` (`KismetStringLibrary.Concat_StrStr` "Pridal som do active quests, teraz mam: " (`KismetStringLibrary.Conv_IntToString` (`KismetArrayLibrary.Array_Length` _activequests))))
        (set `local.TempProgress` (`self.QuestProgress`))
        (`BlueprintMapLibrary.Map_Add` _tempprogress QuestID)
        (set `self.QuestProgress` _tempprogress)
        (bind _returnvalue_2 (`|CreateWidget` "/Game/QuestLog/Widgets/WG_StartedQuest.WG_StartedQuest_C" null _returnvalue))
        (set `self.ActiveWidget` _returnvalue_2)
        (`UserWidget.AddToViewport` _returnvalue_2 0)))
    (else
      (`KismetSystemLibrary.PrintString` "Uz zacal"))))

(fn `UpdateObjectiveCompletion`
  (params (QuestID :type Name) (ObejctiveID :type Name))
  (returns (Completed :type Boolean))
  (locals (TempObjectives :type "Array of /Game/QuestLog/Structs/S_QuestObjectives Structure"))
  (for (_array_element _array_index) (`self.ActiveQuests`)
    (bind (_questid _title _iscompleted _description _objectives) (break `/Game/QuestLog/Structs/S_QuestData` _array_element))
    (set `local.TempObjectives` _objectives)
    (if (== _questid QuestID)
      (for (_array_element_2 _array_index_2) (`.Objectives_27_DB1C4EAF429E6CEAACA8E8B6823740B7` (break `/Game/QuestLog/Structs/S_QuestData` _array_element))
        (if (== (`.ObjectiveID_7_4D4F38A74C8366879E3010A40201A81D` (break `/Game/QuestLog/Structs/S_QuestObjectives` _array_element_2)) ObejctiveID)
          (bind (_objectiveid _description_2 _iscompleted_2 _objectivetype _targetdata _optional _canbecompletedinanyorder) (break `/Game/QuestLog/Structs/S_QuestObjectives` _array_element_2))
          (`KismetArrayLibrary.Array_Set` (`local.TempObjectives`) _array_index_2 (make `/Game/QuestLog/Structs/S_QuestObjectives` _objectiveid _description_2 true _objectivetype _targetdata _optional _canbecompletedinanyorder))
          (bind (_questid_2 _title_2 _iscompleted_3 _description_3 _objectives_2 _isrepeatable _autostart _rewards) (break `/Game/QuestLog/Structs/S_QuestData` _array_element))
          (`KismetArrayLibrary.Array_Set` (`self.ActiveQuests`) _array_index (make `/Game/QuestLog/Structs/S_QuestData` _questid_2 _title_2 true _description_3 (`local.TempObjectives`) _isrepeatable _autostart _rewards))
          (bind _completed (`self.CheckQuestCompleted` _questid_2))
          (return _completed)))
      (return false)))
  (return false))

(fn `UserConstructionScript`)