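; BP_Door is an interactable prison-cell-style door that slides vertically to open and close.
; Interact calls OpenDoor or CloseDoor based on IsOpen, or plays a lock sound while the door is moving.
; One timeline, played or reversed, drives the door's relative Z, with a movement sound at each start.
; IsMoving clears through a fixed Delay on the timeline's Update rather than its Finished output.
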(event `OpenDoor`
  (set `self.IsMoving` true)
  (set `self.IsOpen` true)
  (`GameplayStatics.PlaySoundAtLocation` "/Game/Interactibles/Prison_Cell_Door__mp3cut_net_.Prison_Cell_Door__mp3cut_net_" (`self.K2_GetActorLocation`) (struct) 1.0 1.0 0.0 null null null null)
  (bind (_direction _updown) (`Timeline|OpenDoorTimeline` :!label _label)
    (:`Update`
      (`SceneComponent.K2_SetRelativeLocation` (`self.Door`) (`KismetMathLibrary.MakeVector` 0.0 0.0 _updown) false false)
      (`KismetSystemLibrary.Delay` 2.0)
      (set `self.IsMoving` false))))

(event `CloseDoor`
  (set `self.IsMoving` true)
  (set `self.IsOpen` false)
  (`GameplayStatics.PlaySoundAtLocation` "/Game/Interactibles/Prison_Cell_Door__mp3cut_net_.Prison_Cell_Door__mp3cut_net_" (`self.K2_GetActorLocation`) (struct) 1.0 1.0 0.0 null null null null)
  (goto _label :!via `Reverse`))

(event `/Game/InteractionSystem/BPI_interactible.Interact`
  (params (Interactor :type "Actor Object Reference"))
  (if (`self.IsMoving`)
    (`GameplayStatics.PlaySoundAtLocation` "/Game/Interactibles/Door_Lock_Sound_Effect_1_No_Copyright_Sounds_Sound_Effect_HD_.Door_Lock_Sound_Effect_1_No_Copyright_Sounds_Sound_Effect_HD_" (`self.K2_GetActorLocation`) (struct) 1.0 1.0 0.0 null null null null)
    (elif (`self.IsOpen`)
      (`self.CloseDoor`)
      (else
        (`self.OpenDoor`)))))

(fn `CanBeIntreracted`
  (returns (CanBeInteracted :type Boolean))
  (return true))

(fn `GetInteractionType`
  (returns (NewParam :type "/Game/InteractionSystem/InterctionTypes Enum"))
  (return "NewEnumerator1"))

(fn `UserConstructionScript`)