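; BP_Chest is an interactable chest that opens once when the player interacts with it.
; Interact plays the non-looping Chest_Open animation on the Chest component and sets IsOpen.
; CanBeIntreracted reports true only while the chest is closed, and GetInteractionType returns a fixed enum value.
; The file contains no logic for closing the chest or granting contents.
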(event `/Game/InteractionSystem/BPI_interactible.Interact`
  (params (Interactor :type "Actor Object Reference"))
  (if (not (`self.IsOpen`))
    (`SkeletalMeshComponent.PlayAnimation` (`self.Chest`) "/Game/Interactibles/Chest/Chest_Open.Chest_Open" false)
    (set `self.IsOpen` true)))

(fn `CanBeIntreracted`
  (returns (CanBeInteracted :type Boolean))
  (return (not (`self.IsOpen`))))

(fn `GetInteractionType`
  (returns (NewParam :type "/Game/InteractionSystem/InterctionTypes Enum"))
  (return "NewEnumerator0"))

(fn `UserConstructionScript`)