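; BP_Simon is a Simon Says puzzle controller that starts when a player enters its box and opens a door once won.
; Each level builds a random note sequence, plays it on linked stand actors, then checks player notes, replaying a new sequence on mistakes.
; Start and win complete SearchTheCastle objectives through BP_ServiceManager, and winning then starts SaveThePrincess.
; The construction script caps note counts to the stand count for levels without duplicates.
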(event `self.ReceiveBeginPlay`
  ;[1 1 1] On Begin Play, set Reference in stands
  (for _array_element (`self.Stands`)
    (`/Engine/EditorBlueprintResources/StandardMacros.IsValid` _array_element
      (:`Is Valid`
        (set `/Game/SimonSays/_Main/Blueprints/BP_Stand.SimonNainReference` self _array_element)
        (set `self.PlayerWon` false))
      (:`Is Not Valid`
        (`KismetSystemLibrary.PrintString` "Forgot To add stands!!!" true true (struct :`R` 0.977732 :`G` 1.0 :`A` 1.0))))))

(event `AddNote`
  (bind ((`NumOfNodes_6_BE6F19BF452E411260B1D691BBC7433E` _numofnodes) (`CanDuplicateNotes_10_17CD42AA4D1DC96FE51EA89F269D9797` _canduplicatenotes)) (break `/Game/SimonSays/_Main/Blueprints/SimonLevelStruct` (`|GetArrayItem` (`self.LevelSetting`) (`self.CurrentLevel`))))
  (bind _returnvalue (`KismetMathLibrary.RandomIntegerInRange` 0 (- (`KismetArrayLibrary.Array_Length` (`self.Stands`)) 1)))
  ;[1 1 1] Create Squence
  (if (> (`KismetArrayLibrary.Array_Length` (`self.Stands`)) 0) :!label _label
    (if _canduplicatenotes
      (`KismetArrayLibrary.Array_Add` (`self.SimonSequence`) _returnvalue)
      (else
        (`KismetArrayLibrary.Array_AddUnique` (`self.SimonSequence`) _returnvalue)))
    (if (< (`KismetArrayLibrary.Array_Length` (`self.SimonSequence`)) _numofnodes)
      (`self.AddNote`))))

(event `CreateSimonSequence`
  ;[1 1 1] Create Squence
  (`KismetArrayLibrary.Array_Clear` (`self.SimonSequence`))
  (goto _label))

(event `self.Box.OnComponentBeginOverlap`
  (params (OverlappedComponent :type "PrimitiveComponent Object Reference") (OtherActor :type "Actor Object Reference") (OtherComp :type "PrimitiveComponent Object Reference") (OtherBodyIndex :type Integer) (bFromSweep :type Boolean) (SweepResult :type "HitResult Structure (by ref)"))
  ;[1 1 1] Overlap
  (if (and (`KismetSystemLibrary.DoesImplementInterface` OtherActor "/Game/SimonSays/_Main/Blueprints/BPI_Player.BPI_Player_C") (not (`self.isPlaying`)))
    (if (not (`self.PlayerWon`))
      (set `self.isPlaying` true)
      (`self.StartLevel`)
      (bind _returnvalue (`|GetDataTableRow` "/Game/QuestLog/DataTable/DT_quest.DT_quest" "SearchTheCastle")
        (:`then`
          (bind _returnvalue_2 (`GameplayStatics.GetActorOfClass` "/Game/QuestLog/BPS/BP_ServiceManager.BP_ServiceManager_C"))
          (bind (_questid _title _iscompleted _description _objectives) (break `/Game/QuestLog/Structs/S_QuestData` _returnvalue))
          (message `/Game/QuestLog/Interfaces/INT_ServiceManager.SM_CompleteObjective` _returnvalue_2 _questid (`.ObjectiveID_7_4D4F38A74C8366879E3010A40201A81D` (break `/Game/QuestLog/Structs/S_QuestObjectives` (`|GetArrayItem` _objectives)))))))))

(event `StartLevel`
  (bind ((`NumOfNodes_6_BE6F19BF452E411260B1D691BBC7433E` _numofnodes) (`TimeBetweenNotes_9_2695045E4E14155ACF55DABA4D6813CC` _timebetweennotes)) (break `/Game/SimonSays/_Main/Blueprints/SimonLevelStruct` (`|GetArrayItem` (`self.LevelSetting`) (`self.CurrentLevel`))))
  ;[1 1 1] Start Level
  (`KismetArrayLibrary.Array_Clear` (`self.PlayerSequence`))
  (set `self.CurendNote` 0)
  (set `self.isPlayersTurn` false)
  (`self.CreateSimonSequence`)
  (if (< (`KismetArrayLibrary.Array_Length` (`self.SimonSequence`)) _numofnodes)
    (`KismetSystemLibrary.Delay` 0.2)
    (`self.AddNote`)
    (else
      (`KismetSystemLibrary.Delay` _timebetweennotes)
      (`self.PlaySimonSequence`))))

(event `PlaySimonSequence`
  ;[1 1 1] Play simulation
  (`/Game/SimonSays/_Main/Blueprints/BP_Stand.PlayNode` (`|GetArrayItem` (`self.Stands`) (`|GetArrayItem` (`self.SimonSequence`) (`self.CurendNote`))))
  (`KismetSystemLibrary.Delay` (`.TimeBetweenNotes_9_2695045E4E14155ACF55DABA4D6813CC` (break `/Game/SimonSays/_Main/Blueprints/SimonLevelStruct` (`|GetArrayItem` (`self.LevelSetting`) (`self.CurrentLevel`)))))
  (`/Engine/EditorBlueprintResources/StandardMacros.IncrementInt` (`self.CurendNote`)
    (:`  `
      (if (< (`self.CurendNote`) (`KismetArrayLibrary.Array_Length` (`self.SimonSequence`)))
        (`self.PlaySimonSequence`)
        (else
          (set `self.isPlayersTurn` true))))))

(event `PlayerPlayedNote`
  (params (Note :type Integer))
  (bind _currentlevel (`self.CurrentLevel`))
  ;[1 1 1] Player Played note
  (set `self.isPlayersTurn` false)
  (bind _returnvalue (`KismetArrayLibrary.Array_Add` (`self.PlayerSequence`) Note))
  (if (== Note (`|GetArrayItem` (`self.SimonSequence`) _returnvalue))
    (`/Game/SimonSays/_Main/Blueprints/BP_Stand.PlayNode` (`|GetArrayItem` (`self.Stands`) Note))
    (set `self.isPlayersTurn` true)
    (if (<= (`KismetArrayLibrary.Array_Length` (`self.SimonSequence`)) (`KismetArrayLibrary.Array_Length` (`self.PlayerSequence`)))
      (if (< _currentlevel (`KismetArrayLibrary.Array_LastIndex` (`self.LevelSetting`)))
        (`/Engine/EditorBlueprintResources/StandardMacros.IncrementInt` _currentlevel
          (:`  `
            (`GameplayStatics.PlaySoundAtLocation` "/Game/SimonSays/_Main/Sound/taranp_success.taranp_success" (0.0 0.0 0.0) (struct) 1.0 1.0 0.0 null null null null)
            (`self.StartLevel`)))
        (else
          (set `self.PlayerWon` true)
          (`/Game/Interactibles/BP_PuzzleDoor.OpenDoor` (`self.PuzzleDoor`))
          (bind _returnvalue_2 (`|GetDataTableRow` "/Game/QuestLog/DataTable/DT_quest.DT_quest" "SearchTheCastle")
            (:`then`
              (bind _returnvalue_3 (`GameplayStatics.GetActorOfClass` "/Game/QuestLog/BPS/BP_ServiceManager.BP_ServiceManager_C"))
              (bind (_questid _title _iscompleted _description _objectives) (break `/Game/QuestLog/Structs/S_QuestData` _returnvalue_2))
              (message `/Game/QuestLog/Interfaces/INT_ServiceManager.SM_CompleteObjective` _returnvalue_3 _questid (`.ObjectiveID_7_4D4F38A74C8366879E3010A40201A81D` (break `/Game/QuestLog/Structs/S_QuestObjectives` (`|GetArrayItem` _objectives 1))))
              (`KismetSystemLibrary.Delay` 2.0)
              (bind _returnvalue_4 (`|GetDataTableRow` "/Game/QuestLog/DataTable/DT_quest.DT_quest" "SaveThePrincess")
                (:`then`
                  (bind _returnvalue_5 (`GameplayStatics.GetActorOfClass` "/Game/QuestLog/BPS/BP_ServiceManager.BP_ServiceManager_C"))
                  (`/Game/QuestLog/Interfaces/INT_ServiceManager.SM_StartQuest` _returnvalue_5 (`.QuestID_8_D0F829F54632ABB1EF689CB21D7A8BD5` (break `/Game/QuestLog/Structs/S_QuestData` _returnvalue_4))))))))))
    (else
      (for _array_element (`self.Stands`)
        (`/Game/SimonSays/_Main/Blueprints/BP_Stand.PlayError` _array_element))
      (`self.StartLevel`))))

(fn `UserConstructionScript`
  (bind _returnvalue (`KismetArrayLibrary.Array_Length` (`self.Stands`)))
  (for (_array_element _array_index) (`self.LevelSetting`)
    (bind ((`NumOfNodes_6_BE6F19BF452E411260B1D691BBC7433E` _numofnodes) (`CanDuplicateNotes_10_17CD42AA4D1DC96FE51EA89F269D9797` _canduplicatenotes)) (break `/Game/SimonSays/_Main/Blueprints/SimonLevelStruct` _array_element))
    (if _canduplicatenotes
      _
      (elif (> _numofnodes _returnvalue)
        (bind _structout (setmembers `/Game/SimonSays/_Main/Blueprints/SimonLevelStruct` :`StructRef` _array_element :`NumOfNodes` _returnvalue))
        (`KismetArrayLibrary.Array_Set` (`self.LevelSetting`) _array_index _structout)))))