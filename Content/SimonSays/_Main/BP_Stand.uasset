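; BP_Stand is a colored stand in the Simon Says game that lights up and plays its sound when activated.
; The construction script creates a dynamic material on the capsule and applies the stand's color.
; BeginPlay assigns the sound, and interaction from an actor implementing BPI_Player calls PlayNode.
; PlayNode plays the audio and raises the material's Intensity for a short delay, then resets both.
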(event `self.ReceiveBeginPlay`
  (`AudioComponent.SetSound` (`self.Audio`) (`self.Sound`)))

(event `/Game/SimonSays/_Main/Blueprints/BPI_Puzzle.OnInteract`
  (params (Actorr :type "Actor Object Reference"))
  (if (`KismetSystemLibrary.DoesImplementInterface` Actorr "/Game/SimonSays/_Main/Blueprints/BPI_Player.BPI_Player_C")
    (if true
      (`self.PlayNode`))))

(event `PlayNode`
  (`AudioComponent.Play` (`self.Audio`) 0.0)
  (`MaterialInstanceDynamic.SetScalarParameterValue` (`self.DynMat`) "Intensity" 1.0)
  (`KismetSystemLibrary.Delay` 0.65)
  (`MaterialInstanceDynamic.SetScalarParameterValue` (`self.DynMat`) "Intensity" 0.0)
  (`AudioComponent.Stop` (`self.Audio`)))

(fn `UserConstructionScript`
  (bind _returnvalue (`PrimitiveComponent.CreateDynamicMaterialInstance` (`self.Capsule`) 0 "/Game/SimonSays/_Main/Materials/M_Color.M_Color" "None"))
  (bind _output_get (set `self.DynMat` _returnvalue))
  (`MaterialInstanceDynamic.SetVectorParameterValue` _output_get "Color" (`self.Color`)))