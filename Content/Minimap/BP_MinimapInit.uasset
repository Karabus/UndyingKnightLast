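; Minimap initializer actor that sets up the minimap widget and the player and enemy markers when play begins.
; BeginPlay adds the widget to the viewport, then finds all actors tagged Player or Enemy.
; Each gets a matching marker actor spawned at its location and attached to follow it.
; The first static mesh component of each tagged actor is hidden from scene capture.
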(event `self.ReceiveBeginPlay`
  ;[1 1 1] Vytvorenie Minimapy
  (bind _returnvalue (`|CreateWidget` "/Game/Minimap/WigetMinimap.WigetMinimap_C"))
  (bind _output_get (set `self.NewVar` _returnvalue))
  (`UserWidget.AddToViewport` _output_get 0)
  (`self.CreateMinimapPlayer`)
  (`self.CreateMinimapEnemy`))

(fn `CreateMinimapEnemy`
  (bind _outactors (`GameplayStatics.GetAllActorsWithTag` "Enemy"))
  (for _array_element _outactors
    (bind _returnvalue (`|SpawnActorFromClass` "/Game/Minimap/BP_Minimap_Enemy.BP_Minimap_Enemy_C" (`KismetMathLibrary.MakeTransform` (`self.K2_GetActorLocation` _array_element)) "Undefined" "MultiplyWithRoot" null null))
    (`self.K2_AttachToActor` _returnvalue _array_element "None" "KeepWorld" "KeepWorld" "KeepWorld" true)
    (`PrimitiveComponent.SetHiddenInSceneCapture` (`|GetArrayItem` (`self.K2_GetComponentsByClass` _array_element "/Script/Engine.StaticMeshComponent")) true)))

(fn `CreateMinimapPlayer`
  (bind _outactors (`GameplayStatics.GetAllActorsWithTag` "Player"))
  (for _array_element _outactors
    (bind _returnvalue (`|SpawnActorFromClass` "/Game/Minimap/BP_Minimap_Player.BP_Minimap_Player_C" (`KismetMathLibrary.MakeTransform` (`self.K2_GetActorLocation` _array_element)) "Undefined" "MultiplyWithRoot" null null))
    (`self.K2_AttachToActor` _returnvalue _array_element "None" "KeepWorld" "KeepWorld" "KeepWorld" true)
    (`PrimitiveComponent.SetHiddenInSceneCapture` (`|GetArrayItem` (`self.K2_GetComponentsByClass` _array_element "/Script/Engine.StaticMeshComponent")) true)))

(fn `UserConstructionScript`)