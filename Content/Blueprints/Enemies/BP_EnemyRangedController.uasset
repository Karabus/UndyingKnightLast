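; AI controller for ranged enemies that runs their behavior tree and feeds perception results into its blackboard.
; On possess it sets up the ranged-enemy blackboard and starts the behavior tree.
; Sight stimuli set or clear the target actor, while successfully sensed sounds store an investigate location and raise a flag for it.
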(event `self.ReceivePossess`
  (params (PossessedPawn :type "Pawn Object Reference"))
  (bind _blackboardcomponent (`self.UseBlackboard` "/Game/BB_EnemyRanged.BB_EnemyRanged"))
  (set `self.BBComp` _blackboardcomponent)
  (`self.RunBehaviorTree` "/Game/BT_EnemyRanged.BT_EnemyRanged"))

(event `self.AIPerception.OnTargetPerceptionUpdated`
  (params (Actor :type "Actor Object Reference") (Stimulus :type "AIStimulus Structure"))
  (bind (_age _expirationage _strength _stimuluslocation _receiverlocation _tag _bsuccessfullysensed) (break `AIStimulus` Stimulus))
  (bind _bbcomp (`self.BBComp`))
  (`/Engine/EditorBlueprintResources/StandardMacros.IsValid` (`self.BBComp`)
    (:`Is Valid`
      (bind _returnvalue (`AIPerceptionSystem.GetSenseClassForStimulus` Stimulus))
      (`|ExecutionSequence`
        (:`then_0`
          (if (== _returnvalue "/Script/AIModule.AISense_Sight")
            (if _bsuccessfullysensed
              (`BlackboardComponent.SetValueAsObject` _bbcomp "TargetActor" Actor)
              (else
                (`BlackboardComponent.ClearValue` _bbcomp "TargetActor")))))
        (:`then_1`
          (if (== _returnvalue "/Script/AIModule.AISense_Hearing")
            (if _bsuccessfullysensed
              (`BlackboardComponent.SetValueAsVector` _bbcomp "InvestigateLocation" _stimuluslocation)
              (`BlackboardComponent.SetValueAsBool` _bbcomp "HasInvestigateLocation" true))))))))

(fn `UserConstructionScript`)