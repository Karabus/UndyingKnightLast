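; AI controller for enemies that runs the enemy behavior tree and feeds perception results into its blackboard.
; On possess it sets up the enemy blackboard and starts the tree.
; Perception updates branch by sense: sight sets the target actor and clears it when sight is lost.
; Hearing records the stimulus location and flags it for investigation, leaving any clearing of that flag to elsewhere.
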(event `self.ReceivePossess`
  (params (PossessedPawn :type "Pawn Object Reference"))
  (bind _blackboardcomponent (`self.UseBlackboard` "/Game/BB_Enemy.BB_Enemy"))
  (set `self.BB_Comp` _blackboardcomponent)
  (`self.RunBehaviorTree` "/Game/BT_Enemy.BT_Enemy"))

(event `self.AIPerception.OnTargetPerceptionUpdated`
  (params (Actor :type "Actor Object Reference") (Stimulus :type "AIStimulus Structure"))
  (bind (_age _expirationage _strength _stimuluslocation _receiverlocation _tag _bsuccessfullysensed) (break `AIStimulus` Stimulus))
  (bind _bb_comp (`self.BB_Comp`))
  (`/Engine/EditorBlueprintResources/StandardMacros.IsValid` (`self.BB_Comp`)
    (:`Is Valid`
      (bind _returnvalue (`AIPerceptionSystem.GetSenseClassForStimulus` Stimulus))
      (`|ExecutionSequence`
        (:`then_0`
          (if (== _returnvalue "/Script/AIModule.AISense_Sight")
            (if _bsuccessfullysensed
              (`BlackboardComponent.SetValueAsObject` _bb_comp "TargetActor" Actor)
              (else
                (`BlackboardComponent.ClearValue` _bb_comp "TargetActor")))))
        (:`then_1`
          (if (== _returnvalue "/Script/AIModule.AISense_Hearing")
            (if _bsuccessfullysensed
              (`BlackboardComponent.SetValueAsVector` _bb_comp "InvestigateLocation" _stimuluslocation)
              (`BlackboardComponent.SetValueAsBool` _bb_comp "HasInvestigateLocation" true))))))))

(fn `UserConstructionScript`)