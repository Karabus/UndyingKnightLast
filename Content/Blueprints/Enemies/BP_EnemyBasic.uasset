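; Basic enemy that wanders between random nearby points, chases the player within range and attacks up close.
; Tick runs distance checks that start or stop a looping damage timer and drive rotation and swept offset movement, without AI controller or navigation.
; Taking damage briefly swaps to a hit material; at zero health it stops attacking, disables collision, spawns an apple and destroys itself.
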(event `self.ReceiveBeginPlay`
  ;[1 1 1] Init
  (set `self.Health` (`self.MaxHealth`))
  (`PrimitiveComponent.SetMaterial` (`self.Body`) 0 (`self.NormalMat`))
  (bind _asbpfirst_person_character (cast `/Game/Pohyb/BPFirstPersonCharacter` (`GameplayStatics.GetPlayerCharacter` 0)))
  (set `self.PlayerRef` _asbpfirst_person_character)
  (`self.SetTargetPoint`))

(event `self.ReceiveTick`
  (params (DeltaSeconds :type "Float (single-precision)"))
  ;[1 1 1] Hlavná slučka programu
  (bind (_inchaserange _distance _inattackrange) (`self.EnemyIsClose`))
  (bind _output_get (set `self.InAttackRange` _inattackrange))
  (`|ExecutionSequence`
    (:`then_0`
      (if _output_get
        (`self.StartAttacking`)
        (else
          (`self.StopAttacking`))))
    (:`then_1`
      (bind _output_get_2 (set `self.IsChasing` (or _inchaserange _inattackrange)))
      (if _output_get_2
        (`self.UpdateRotationToPlayer`)
        (else
          (`self.RotateToTargetPoint` 0.0)))
      (`self.UpdateMovement`))))

(event `self.ReceiveAnyDamage`
  (params (Damage :type "Float (single-precision)") (DamageType :type "DamageType Object Reference") (InstigatedBy :type "Controller Object Reference") (DamageCauser :type "Actor Object Reference"))
  ;[1 1 1] Logika hittovania enemy
  (if (not (`self.IsDead`))
    (set `self.Health` (- (`self.Health`) Damage))
    (`PrimitiveComponent.SetMaterial` (`self.Body`) 0 (`self.HitMat`))
    (`KismetSystemLibrary.K2_SetTimerDelegate` (delegate `ResetHitMaterial`) 0.1 :!label _label)
    (if (<= (`self.Health`) 0.0)
      (`self.Die`))))

(event `ResetHitMaterial`
  ;[1 1 1] Logika hittovania enemy
  (`PrimitiveComponent.SetMaterial` (`self.Body`) 0 (`self.NormalMat`))
  (goto _label))

(event `Die`
  ;[1 1 1] Zabitie Enemy a drop jablka
  (`self.StopAttacking`)
  (set `self.IsDead` true)
  (set `self.CanDamage` false)
  (`PrimitiveComponent.SetCollisionEnabled` (`self.Body`) "NoCollision")
  (`KismetSystemLibrary.Delay` 0.2)
  (`|SpawnActorFromClass` "/Game/Inventory/Items/Apple.Apple_C" (`KismetMathLibrary.Conv_VectorToTransform` (`self.K2_GetActorLocation`)) "Undefined" "MultiplyWithRoot" null null)
  (`self.K2_DestroyActor`))

(event `DoAttack`
  ;[1 1 1] Logika útočenia
  (if (not (`self.IsDead`))
    (`/Engine/EditorBlueprintResources/StandardMacros.IsValid` (`self.PlayerRef`)
      (:`Is Valid`
        (`GameplayStatics.ApplyDamage` (`self.PlayerRef`) (`self.AttackDamage`) null self)))))

(event `StartAttacking`
  ;[1 1 1] Logika útočenia
  (if (not (`self.IsAttacking`))
    (set `self.IsAttacking` true)
    (`self.DoAttack`)
    (bind _returnvalue (`KismetSystemLibrary.K2_SetTimerDelegate` (delegate `DoAttack`) (`self.AttackInterval`) true))
    (set `self.AttackTimerHandle` _returnvalue)))

(event `StopAttacking`
  ;[1 1 1] Stop Attacking
  (`KismetSystemLibrary.K2_ClearAndInvalidateTimerHandle` (`self.AttackTimerHandle`))
  (set `self.IsAttacking` false))

(fn `EnemyIsClose`
  (returns (InChaseRange :type Boolean) (Distance :type "Vector Structure") (InAttackRange :type Boolean))
  (bind _returnvalue (- (`self.K2_GetActorLocation` (`self.PlayerRef`)) (`self.K2_GetActorLocation`)))
  (bind _returnvalue_2 (`KismetMathLibrary.VSize` _returnvalue))
  (return (< _returnvalue_2 (`self.ChaseRange`)) _returnvalue (<= _returnvalue_2 (`self.AttackRange`))))

(fn `RotateToTargetPoint`
  (params (NewParam :type "Float (double-precision)"))
  (`self.K2_SetActorRotation` (`KismetMathLibrary.RInterpTo` (`self.K2_GetActorRotation`) (`KismetMathLibrary.MakeRotator` 0.0 0.0 (.yaw (`KismetMathLibrary.FindLookAtRotation` (`self.K2_GetActorLocation`) (`self.TargetPoint`)))) NewParam (`self.TurnSpeed`))))

(fn `SetTargetPoint`
  (bind _returnvalue (`self.K2_GetActorLocation`))
  (set `self.TargetPoint` (`KismetMathLibrary.MakeVector` (.x (+ _returnvalue (* (`KismetMathLibrary.RandomUnitVector`) (`self.Range`)))) (.y (+ _returnvalue (* (`KismetMathLibrary.RandomUnitVector`) (`self.Range`)))) (.z _returnvalue))))

(fn `UpdateMovement`
  (bind _returnvalue (`GameplayStatics.GetWorldDeltaSeconds`))
  (bind _returnvalue_2 (- (`self.TargetPoint`) (`self.K2_GetActorLocation`)))
  (if (`self.IsChasing`)
    (if (not (`self.InAttackRange`))
      (`self.K2_AddActorWorldOffset` (* (* (`KismetMathLibrary.Normal` (- (`self.K2_GetActorLocation` (`self.PlayerRef`)) (`self.K2_GetActorLocation`))) (`self.Speed`)) _returnvalue) true))
    (else
      (`self.K2_AddActorWorldOffset` (* (`KismetMathLibrary.Normal` _returnvalue_2) (`self.Speed`) _returnvalue) true)
      (if (< (`KismetMathLibrary.VSize` _returnvalue_2) 100.0)
        (`self.SetTargetPoint`)))))

(fn `UpdateRotationToPlayer`
  (`self.K2_SetActorRotation` (`KismetMathLibrary.RInterpTo` (`self.K2_GetActorRotation`) (`KismetMathLibrary.FindLookAtRotation` (`self.K2_GetActorLocation`) (`self.K2_GetActorLocation` (`self.PlayerRef`))) (`GameplayStatics.GetWorldDeltaSeconds`) (`self.TurnSpeed`))))

(fn `UserConstructionScript`)