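; BP_EnemyRanged is an AI enemy that damages the first-person player with a forward sphere trace during its shoot montage.
; Aggro and attack-range spheres feed target and range keys to the BP_EnemyAIController blackboard.
; Interrupted or out-of-range attacks start a timer that restores CanAttack; damage drives throttled hit reacts or death, which stops AI.
; Manual wander, chase and rotation helpers are defined but never called here.
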(event `PerformAttackHit`
  (bind _returnvalue (+ (+ (`self.K2_GetActorLocation`) (* (`self.GetActorForwardVector`) 60.0)) (0.0 0.0 50.0)))
  (if (not (`self.IsDead`))
    (if (not (`self.DidHitThisAttack`))
      (bind _outhit (`KismetSystemLibrary.SphereTraceSingleForObjects` _returnvalue (+ _returnvalue (* (`self.GetActorForwardVector`) (`KismetMathLibrary.FClamp` (`self.GetDistanceTo` (`GameplayStatics.GetPlayerCharacter` 0)) 120.0 260.0))) 45.0 (`|MakeArray` "ObjectTypeQuery3" :!type "EObjectTypeQuery Enum") false (`|MakeArray` self :!type "Actor Object Reference") "ForDuration"))
      (bind _asbpfirst_person_character (cast `/Game/Pohyb/BPFirstPersonCharacter` (`.HitActor` (`GameplayStatics.BreakHitResult` _outhit))))
      (`GameplayStatics.ApplyDamage` _asbpfirst_person_character 10.0 (`self.GetController`) self)
      (set `self.DidHitThisAttack` true))))

(event `TryContinueAttack`
  (if (`self.IsDead`)
    _
    (elif (not (<= (`self.GetDistanceTo` (`GameplayStatics.GetPlayerCharacter` 0) self) (`self.AttackRange`)))
      (`AnimInstance.Montage_Stop` (`SkeletalMeshComponent.GetAnimInstance` (`self.Mesh`)) 0.0 (`self.ShootMontage`))
      (`self.OnAttackEnded`))))

(event `ResetCanAttack`
  (bind _asbp_enemy_aicontroller (cast `/Game/Blueprints/Enemies/BP_EnemyAIController` (`self.GetController`)))
  (`BlackboardComponent.SetValueAsBool` (`AIController.Blackboard` _asbp_enemy_aicontroller) "CanAttack" true))

(event `self.ReceiveBeginPlay`
  (bind _asbp_enemy_aicontroller (cast `/Game/Blueprints/Enemies/BP_EnemyAIController` (`self.GetController`)))
  (`BlackboardComponent.SetValueAsBool` (`AIController.Blackboard` _asbp_enemy_aicontroller) "CanShoot" true)
  (set `self.Health` (`self.MaxHealth`)))

(event `PlayHitReact`
  (if (`self.IsDead`)
    _
    (elif (`self.CanHitReact`)
      (set `self.CanHitReact` false)
      (`|PlayMontage` (`self.Mesh`) (`self.HitMontage`)
        (:`then`
          (`KismetSystemLibrary.Delay` (`self.HitReactCooldown`))
          (set `self.CanHitReact` true))))))

(event `self.ReceiveAnyDamage`
  (params (Damage :type "Float (single-precision)") (DamageType :type "DamageType Object Reference") (InstigatedBy :type "Controller Object Reference") (DamageCauser :type "Actor Object Reference"))
  ;[1 1 1] Logika hittovania enemy
  (if (not (`self.IsDead`))
    (bind _output_get (set `self.Health` (`KismetMathLibrary.FClamp` (- (`self.Health`) Damage) 0.0 (`self.MaxHealth`))))
    (if (<= _output_get 0.0)
      (`self.Die`)
      (else
        (`self.PlayHitReact`)))))

(event `Die`
  (if (not (`self.IsDead`))
    (set `self.IsDead` true)
    (set `self.CanHitReact` false)
    (bind _asbp_enemy_aicontroller (cast `/Game/Blueprints/Enemies/BP_EnemyAIController` (`self.GetController`)))
    (`Controller.StopMovement` _asbp_enemy_aicontroller)
    (`BrainComponent.StopLogic` (`AIController.BrainComponent` _asbp_enemy_aicontroller) "Dead")
    (`|PlayMontage` (`self.Mesh`) (`self.DeathMontage`)
      (:`then`
        (bind _blackboard (`AIController.Blackboard` _asbp_enemy_aicontroller))
        (`BlackboardComponent.ClearValue` _blackboard "TargetActor")
        (`BlackboardComponent.SetValueAsBool` _blackboard "CanAttack" false)
        (`PrimitiveComponent.SetCollisionEnabled` (`self.CapsuleComponent`) "NoCollision")
        (`PrimitiveComponent.SetCollisionEnabled` (`self.AggroSphere`) "NoCollision")
        (`PrimitiveComponent.SetCollisionEnabled` (`self.AttackRangeSphere`) "NoCollision")
        (`self.SetLifeSpan` 4.0)))))

(event `DoAttack`
  (if (not (`self.IsDead`))
    (if (not (`self.IsAttacking`))
      (set `self.IsAttacking` true)
      (set `self.DidHitThisAttack` false)
      (if (not (`AnimInstance.Montage_IsPlaying` (`SkeletalMeshComponent.GetAnimInstance` (`self.Mesh`)) (`self.ShootMontage`)))
        (set `self.DidHitThisAttack` false)
        (`|PlayMontage` (`self.Mesh`) (`self.ShootMontage`)
          (:`OnInterrupted`
            (`self.OnAttackEnded`)))))))

(event `OnAttackEnded`
  (set `self.IsAttacking` false)
  (`self.StartAttackCooldown`))

(event `self.AggroSphere.OnComponentBeginOverlap`
  (params (OverlappedComponent :type "PrimitiveComponent Object Reference") (OtherActor :type "Actor Object Reference") (OtherComp :type "PrimitiveComponent Object Reference") (OtherBodyIndex :type Integer) (bFromSweep :type Boolean) (SweepResult :type "HitResult Structure (by ref)"))
  (bind _asbpfirst_person_character (cast `/Game/Pohyb/BPFirstPersonCharacter` OtherActor))
  (bind _asbp_enemy_aicontroller (cast `/Game/Blueprints/Enemies/BP_EnemyAIController` (`self.GetController`)))
  (`BlackboardComponent.SetValueAsObject` (`AIController.Blackboard` _asbp_enemy_aicontroller) "TargetActor" _asbpfirst_person_character)
  (set `self.InCombat` true))

(event `self.AggroSphere.OnComponentEndOverlap`
  (params (OverlappedComponent :type "PrimitiveComponent Object Reference") (OtherActor :type "Actor Object Reference") (OtherComp :type "PrimitiveComponent Object Reference") (OtherBodyIndex :type Integer))
  (cast `/Game/Pohyb/BPFirstPersonCharacter` OtherActor)
  (bind _asbp_enemy_aicontroller (cast `/Game/Blueprints/Enemies/BP_EnemyAIController` (`self.GetController`)))
  (`BlackboardComponent.ClearValue` (`AIController.Blackboard` _asbp_enemy_aicontroller) "TargetActor")
  (set `self.InCombat` false))

(event `self.AttackRangeSphere.OnComponentBeginOverlap`
  (params (OverlappedComponent :type "PrimitiveComponent Object Reference") (OtherActor :type "Actor Object Reference") (OtherComp :type "PrimitiveComponent Object Reference") (OtherBodyIndex :type Integer) (bFromSweep :type Boolean) (SweepResult :type "HitResult Structure (by ref)"))
  (cast `/Game/Pohyb/BPFirstPersonCharacter` OtherActor)
  (bind _asbp_enemy_aicontroller (cast `/Game/Blueprints/Enemies/BP_EnemyAIController` (`self.GetController`)))
  (`BlackboardComponent.SetValueAsBool` (`AIController.Blackboard` _asbp_enemy_aicontroller) "IsInAttackRange" true))

(event `self.AttackRangeSphere.OnComponentEndOverlap`
  (params (OverlappedComponent :type "PrimitiveComponent Object Reference") (OtherActor :type "Actor Object Reference") (OtherComp :type "PrimitiveComponent Object Reference") (OtherBodyIndex :type Integer))
  (cast `/Game/Pohyb/BPFirstPersonCharacter` OtherActor)
  (bind _asbp_enemy_aicontroller (cast `/Game/Blueprints/Enemies/BP_EnemyAIController` (`self.GetController`)))
  (`BlackboardComponent.SetValueAsBool` (`AIController.Blackboard` _asbp_enemy_aicontroller) "IsInAttackRange" false)
  (set `self.InCombat` false))

(fn `EnemyIsClose`
  (returns (InChaseRange :type Boolean) (Distance :type "Vector Structure") (InAttackRange :type Boolean))
  (bind _returnvalue (- (`self.K2_GetActorLocation` (`self.PlayerRef`)) (`self.K2_GetActorLocation`)))
  (bind _returnvalue_2 (`KismetMathLibrary.VSize` _returnvalue))
  (return (< _returnvalue_2 (`self.ChaseRange`)) _returnvalue (<= _returnvalue_2 (`self.AttackRange`))))

(fn `Rotate to Target Point`
  (params (NewParam :type "Float (double-precision)"))
  (`self.K2_SetActorRotation` (`KismetMathLibrary.RInterpTo` (`self.K2_GetActorRotation`) (`KismetMathLibrary.MakeRotator` 0.0 0.0 (.yaw (`KismetMathLibrary.FindLookAtRotation` (`self.K2_GetActorLocation`) (`self.TargetPoint`)))) NewParam (`self.TurnSpeed`))))

(fn `SetTargetPoint`
  (bind _returnvalue (`self.K2_GetActorLocation`))
  (set `self.TargetPoint` (`KismetMathLibrary.MakeVector` (.x (+ _returnvalue (* (`KismetMathLibrary.RandomUnitVector`) (`self.Range`)))) (.y (+ _returnvalue (* (`KismetMathLibrary.RandomUnitVector`) (`self.Range`)))) (.z _returnvalue))))

(fn `StartAttackCooldown`
  (if (not (`self.IsDead`))
    (`KismetSystemLibrary.K2_ClearTimer` null "RestCanAttack")
    (`KismetSystemLibrary.K2_SetTimer` null "ResetCanAttack" (`self.AttackCooldown`))))

(fn `UpdateMovement`
  (bind _returnvalue (`GameplayStatics.GetWorldDeltaSeconds`))
  (bind _returnvalue_2 (- (`self.TargetPoint`) (`self.K2_GetActorLocation`)))
  (if (`self.IsChasing`)
    (if (not (`self.InAttackRange`))
      (`self.K2_AddActorWorldOffset` (* (* (`KismetMathLibrary.Normal` (- (`self.K2_GetActorLocation` (`self.PlayerRef`)) (`self.K2_GetActorLocation`))) (`self.Speed`)) _returnvalue) true))
    (else
      (`self.K2_AddActorWorldOffset` (* (`KismetMathLibrary.Normal` _returnvalue_2) (`self.Speed`) _returnvalue) true)
      (if (< (`KismetMathLibrary.VSize` _returnvalue_2) 100.0)
        (`self.SetTargetPoint`)))))

(fn `UpdateRotationToPlayer`
  (`self.K2_SetActorRotation` (`KismetMathLibrary.RInterpTo` (`self.K2_GetActorRotation`) (`KismetMathLibrary.FindLookAtRotation` (`self.K2_GetActorLocation`) (`self.K2_GetActorLocation` (`self.PlayerRef`))) (`GameplayStatics.GetWorldDeltaSeconds`) (`self.TurnSpeed`))))

(fn `UserConstructionScript`)