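; BP_Wave is a trigger that starts an enemy wave quest when a BPI_Player actor enters its box.
; The overlap disables the box's collision, spawns BP_EnemyBase actors at one hardcoded location, flags them as wave enemies and starts ClearWave through BP_ServiceManager.
; RemoveEnemy shrinks the tracked array; once empty, it completes ClearWave's first objective and, after a short delay, starts TalkToKnight, both read from DT_quest.
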(event `self.BoxCollision.OnComponentBeginOverlap`
  (params (OverlappedComponent :type "PrimitiveComponent Object Reference") (OtherActor :type "Actor Object Reference") (OtherComp :type "PrimitiveComponent Object Reference") (OtherBodyIndex :type Integer) (bFromSweep :type Boolean) (SweepResult :type "HitResult Structure (by ref)"))
  (if (`KismetSystemLibrary.DoesImplementInterface` OtherActor "/Game/SimonSays/_Main/Blueprints/BPI_Player.BPI_Player_C")
    (`PrimitiveComponent.SetCollisionEnabled` OverlappedComponent "NoCollision")
    (bind _returnvalue (`GameplayStatics.GetActorOfClass` "/Game/QuestLog/BPS/BP_ServiceManager.BP_ServiceManager_C"))
    (set `self.ServiceManager` _returnvalue)
    (for _ (range (+ (`self.EnemyCount`) 1))
      (bind _returnvalue_2 (`|SpawnActorFromClass` "/Game/Blueprints/Enemies/BP_EnemyBase.BP_EnemyBase_C" (`KismetMathLibrary.MakeTransform` (18210.0 7230.0 88.0)) "Undefined" "MultiplyWithRoot" null null))
      (`/Engine/EditorBlueprintResources/StandardMacros.IsValid` _returnvalue_2
        (:`Is Valid`
          (`KismetArrayLibrary.Array_Add` (`self.Enemies`) _returnvalue_2))
        (:`Is Not Valid`
          (`self.K2_DestroyActor` _returnvalue_2))))
    (for _array_element (`self.Enemies`)
      (set `/Game/Blueprints/Enemies/BP_EnemyBase.WaveEnemy` true _array_element))
    (bind _returnvalue_3 (`|GetDataTableRow` "/Game/QuestLog/DataTable/DT_quest.DT_quest" "ClearWave")
      (:`then`
        (message `/Game/QuestLog/Interfaces/INT_ServiceManager.SM_StartQuest` (`self.ServiceManager`) (`.QuestID_8_D0F829F54632ABB1EF689CB21D7A8BD5` (break `/Game/QuestLog/Structs/S_QuestData` _returnvalue_3)))))))

(event `RemoveEnemy`
  (params (NewParam :type "/Game/Blueprints/Enemies/BP_EnemyBase Object Reference"))
  (bind _enemies (`self.Enemies`))
  (`KismetArrayLibrary.Array_RemoveItem` _enemies NewParam)
  (if (`KismetArrayLibrary.Array_IsEmpty` _enemies)
    (bind _returnvalue (`|GetDataTableRow` "/Game/QuestLog/DataTable/DT_quest.DT_quest" "ClearWave")
      (:`then`
        (bind (_questid _title _iscompleted _description _objectives) (break `/Game/QuestLog/Structs/S_QuestData` _returnvalue))
        (message `/Game/QuestLog/Interfaces/INT_ServiceManager.SM_CompleteObjective` (`self.ServiceManager`) _questid (`.ObjectiveID_7_4D4F38A74C8366879E3010A40201A81D` (break `/Game/QuestLog/Structs/S_QuestObjectives` (`|GetArrayItem` _objectives))))
        (`KismetSystemLibrary.Delay` 3.0)
        (bind _returnvalue_2 (`|GetDataTableRow` "/Game/QuestLog/DataTable/DT_quest.DT_quest" "TalkToKnight")
          (:`then`
            (bind _questid_2 (break `/Game/QuestLog/Structs/S_QuestData` _returnvalue_2))
            (message `/Game/QuestLog/Interfaces/INT_ServiceManager.SM_StartQuest` (`self.ServiceManager`) _questid_2)
            (`KismetSystemLibrary.PrintString` (`KismetStringLibrary.Conv_NameToString` _questid_2))))))))

(fn `Decreese Enemy Count`
  (`/Engine/EditorBlueprintResources/StandardMacros.DecrementInt` (`self.EnemyCount`)))

(fn `UserConstructionScript`)